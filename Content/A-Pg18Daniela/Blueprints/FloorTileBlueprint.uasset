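; Endless-runner floor tile for the jetpack game that populates itself with coins and an obstacle.
; The construction script scatters coins within a box's X/Z extents and places one of two randomly chosen child-actor obstacles at a low, medium or high spawn point.
; When the player overlaps PassTrigger, it asks the game mode to add a tile, then destroys itself after a delay.
; GetAttachTransform exposes the endpoint for attaching the next tile.
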(event `self.PassTrigger.OnComponentBeginOverlap`
  (params (OverlappedComponent :type "PrimitiveComponent Object Reference") (OtherActor :type "Actor Object Reference") (OtherComp :type "PrimitiveComponent Object Reference") (OtherBodyIndex :type Integer) (bFromSweep :type Boolean) (SweepResult :type "HitResult Structure (by ref)"))
  ;[1 1 1] adds another floor tile when the player gets to the end of the current floor tile
  (cast `/Game/A-Pg18Daniela/Character/JetPackCharacter` OtherActor)
  (bind _asjet_pack_game_mode (cast `/Game/A-Pg18Daniela/GameModes/JetPackGameMode` (`GameplayStatics.GetGameMode`)))
  (`/Game/A-Pg18Daniela/GameModes/JetPackGameMode.addFloorTile` _asjet_pack_game_mode)
  (`KismetSystemLibrary.Delay` (`self.TimeBeforeDestruction`))
  (`self.K2_DestroyActor`))

(fn `GetAttachTransform`
  (returns (AttachTransform :type "Transform Structure"))
  ;[1 1 1] gets the endpoint of the tile to attach the next tile
  (return (`SceneComponent.K2_GetComponentToWorld` (`self.attachPoint`))))

(fn `SpawnCoins`
  (bind _spawnpickupsarea (`self.spawnPickupsArea`))
  (bind (_boxextent_x _boxextent_y _boxextent_z) (`KismetMathLibrary.BreakVector` (`BoxComponent.BoxExtent` _spawnpickupsarea)))
  ;[1 1 1] Spawns the pick ups randomly in the pick up area
  (for _ (range (`self.minPickUpsInTile`) (+ (`self.maxPickUpsInTile`) 1))
    (`AddComponent|NODE_AddChildActorComponent-1` :`RelativeTransform` (`KismetMathLibrary.Conv_VectorToTransform` (`KismetMathLibrary.RandomPointInBoundingBox` (`SceneComponent.RelativeLocation` _spawnpickupsarea) (`KismetMathLibrary.MakeVector` _boxextent_x 0.0 _boxextent_z))))))

(fn `SpawnObstacle`
  (bind _spawnpoints (`self.SpawnPoints`))
  (bind _output (`|GetArrayItem` _spawnpoints (`KismetMathLibrary.RandomIntegerInRange` 0 (`KismetArrayLibrary.Array_LastIndex` _spawnpoints))))
  ;[1 1 1] spawns an obstacle in one of the spawn points... kinda shot myself in the foot here making the obstacles actors and not comonents, couldn't figure out how to make an array of actors so i had to make a siwtch instead of a get in the array
  (switch `int` (`KismetMathLibrary.RandomIntegerInRange` 0 1)
    (:`Default`
      (`AddComponent|NODE_AddChildActorComponent-2` :`RelativeTransform` _output :!label _label))
    (:`0`
      (`AddComponent|NODE_AddChildActorComponent-0` :`RelativeTransform` _output))
    (:`1`
      (goto _label))))

(fn `StoreSpawnPoints`
  ;[1 1 1] Get all the spawn points and keeps them in an array
  (set `self.SpawnPoints` (`|MakeArray` (`SceneComponent.GetRelativeTransform` (`self.SpawnPointLow`)) (`SceneComponent.GetRelativeTransform` (`self.SpawnPointMedium`)) (`SceneComponent.GetRelativeTransform` (`self.SpawnPointHigh`)))))

(fn `UserConstructionScript`
  (`self.StoreSpawnPoints`)
  (`self.SpawnCoins`)
  (`self.SpawnObstacle`))